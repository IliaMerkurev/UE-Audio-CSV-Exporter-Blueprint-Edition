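; BP_AudioExporter is an actor that records sound events during play and exports them as a CSV-style log.
; BeginPlay adds a header to AudioLog, and AddSoundLog appends a comma-separated entry of time, sound, volume, pan and duration.
; EndPlay joins the entries with an empty separator, adding no line breaks, and writes the string to SaveDir in one write.
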(event `self.ReceiveBeginPlay`
  (`KismetArrayLibrary.Array_Add` (`self.AudioLog`) "time,sound,volume,pan,duration"))

(event `self.ReceiveEndPlay`
  (params (EndPlayReason :type "EEndPlayReason Enum" :default "Destroyed"))
  (`FileSDKBPLibrary.WriteStringToFile` (`self.SaveDir`) (`KismetStringLibrary.JoinStringArray` (`self.AudioLog`) " \n")))

(fn `AddSoundLog`
  (params (Time :type "Float (double-precision)") (Sound :type String) (Volume :type "Float (double-precision)") (Pan :type "Float (double-precision)") (Duration :type "Float (double-precision)"))
  (`KismetArrayLibrary.Array_Add` (`self.AudioLog`) (`KismetStringLibrary.Concat_StrStr` (`KismetStringLibrary.Conv_DoubleToString` Time) "," Sound "," (`KismetStringLibrary.Conv_DoubleToString` Volume) "," (`KismetStringLibrary.Conv_DoubleToString` Pan) "," (`KismetStringLibrary.Conv_DoubleToString` Duration))))

(fn `UserConstructionScript`)